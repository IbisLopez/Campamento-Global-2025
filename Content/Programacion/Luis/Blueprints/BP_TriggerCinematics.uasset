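; BP_TriggerCinematics is a one-shot trigger actor that plays a cinematic when its box component is overlapped.
; The overlap creates a Level Sequence player for the VideoToReproduce variable and starts it, without checking which actor entered.
; It then disables input on the player's BP_ThirdPersonCharacter for a delay equal to the sequence's duration.
; Afterwards it re-enables input and destroys itself.
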(event `self.BoxTriggerCinematic.OnComponentBeginOverlap`
  (params (OverlappedComponent :type "PrimitiveComponent Object Reference") (OtherActor :type "Actor Object Reference") (OtherComp :type "PrimitiveComponent Object Reference") (OtherBodyIndex :type Integer) (bFromSweep :type Boolean) (SweepResult :type "HitResult Structure (by ref)"))
  (bind _outactor (`LevelSequencePlayer.CreateLevelSequencePlayer` (`self.video to reproduce`)))
  (bind _sequenceplayer (`LevelSequenceActor.SequencePlayer` _outactor))
  (`MovieSceneSequencePlayer.Play` _sequenceplayer)
  (bind _asbp_third_person_character (cast `/Game/ThirdPerson/Blueprints/BP_ThirdPersonCharacter` (`GameplayStatics.GetPlayerCharacter` 0)))
  (`self.DisableInput` _asbp_third_person_character null)
  (`KismetSystemLibrary.Delay` (`TimeManagementBlueprintLibrary.Conv_QualifiedFrameTimeToSeconds` (`MovieSceneSequencePlayer.GetDuration` _sequenceplayer)))
  (`self.EnableInput` _asbp_third_person_character null)
  (`self.K2_DestroyActor`))

(fn `UserConstructionScript`)