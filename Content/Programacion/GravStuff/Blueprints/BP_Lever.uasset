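; BP_Lever is an interactable lever that sends a held or released state to the active grid.
; A sphere overlap shows or hides its widget, and leaving the sphere also releases the lever.
; ActivateGlow toggles IsPressed.
; Each state update finds BP_GridManager, matches the actor of its CopiaDelGrid class against five grid references, and calls HoldingLever on the match with 1 or 0.
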(event `self.Sphere.OnComponentBeginOverlap`
  (params (OverlappedComponent :type "PrimitiveComponent Object Reference") (OtherActor :type "Actor Object Reference") (OtherComp :type "PrimitiveComponent Object Reference") (OtherBodyIndex :type Integer) (bFromSweep :type Boolean) (SweepResult :type "HitResult Structure (by ref)"))
  (`SceneComponent.SetVisibility` (`self.Widget`) true false))

(event `self.Sphere.OnComponentEndOverlap`
  (params (OverlappedComponent :type "PrimitiveComponent Object Reference") (OtherActor :type "Actor Object Reference") (OtherComp :type "PrimitiveComponent Object Reference") (OtherBodyIndex :type Integer))
  (`SceneComponent.SetVisibility` (`self.Widget`) false false)
  (set `self.IsPressed` false :!label _label)
  (bind _outactors (`GameplayStatics.GetAllActorsOfClass` "/Game/Programacion/Blueprints/BP_GridManager.BP_GridManager_C" :!label _label_2))
  (bind _output (`|GetArrayItem` _outactors))
  (bind _returnvalue (`GameplayStatics.GetActorOfClass` (`/Game/Programacion/Blueprints/BP_GridManager.CopiaDelGrid` _output)))
  (bind _grid_c1 (`/Game/Programacion/Blueprints/BP_GridManager.Grid C1` _output))
  (`self.Holding Lever` _grid_c1 (== _returnvalue _grid_c1))
  (bind _grid_c2 (`/Game/Programacion/Blueprints/BP_GridManager.Grid C2` _output))
  (`self.Holding Lever` _grid_c2 (== _returnvalue _grid_c2))
  (bind _grid_c3 (`/Game/Programacion/Blueprints/BP_GridManager.Grid C3` _output))
  (`self.Holding Lever` _grid_c3 (== _returnvalue _grid_c3))
  (bind _grid_c4 (`/Game/Programacion/Blueprints/BP_GridManager.Grid C4` _output))
  (`self.Holding Lever` _grid_c4 (== _returnvalue _grid_c4))
  (bind _grid_c5 (`/Game/Programacion/Blueprints/BP_GridManager.Grid C5` _output))
  (`self.Holding Lever` _grid_c5 (== _returnvalue _grid_c5)))

(event `/Game/Programacion/GravStuff/BPI_Interact.ActivateGlow`
  (if (`self.IsPressed`)
    (goto _label)
    (else
      (set `self.IsPressed` true)
      (goto _label_2))))

(fn `Holding Lever`
  (params (Var :type "/Game/Programacion/Blueprints/BP_Grid_NO_MODIFICAR_SOLO_COPIAR Object Reference") (Condition :type Boolean))
  (if Condition
    (if (`self.IsPressed`)
      (`/Game/Programacion/Blueprints/BP_Grid_NO_MODIFICAR_SOLO_COPIAR.HoldingLever` Var 1.0)
      (else
        (`/Game/Programacion/Blueprints/BP_Grid_NO_MODIFICAR_SOLO_COPIAR.HoldingLever` Var 0.0)))
    (else
      (return))))

(fn `UserConstructionScript`)