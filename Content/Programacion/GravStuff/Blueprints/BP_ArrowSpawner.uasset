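; BP_ArrowSpawner is a spawner actor that repeatedly fires BP_FlyingArrow actors from its own location and rotation.
; Tick runs a self-restarting cycle, using the ShootingArrows flag to block overlapping runs during a random delay between configurable bounds.
; Each new arrow receives the spawner's ArrowSpeed, then gets an OnSpawn call after a short delay before the cycle unlocks.
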(event `self.ReceiveBeginPlay`)

(event `self.ReceiveTick`
  (params (DeltaSeconds :type "Float (single-precision)"))
  (if (not (`self.ShootingArrows`))
    (set `self.ShootingArrows` true)
    (`KismetSystemLibrary.Delay` (`KismetMathLibrary.RandomFloatInRange` (`self.minTimeInterval`) (`self.maxTimeInterval`)))
    (bind _returnvalue (`|SpawnActorFromClass` "/Game/Programacion/GravStuff/Blueprints/BP_FlyingArrow.BP_FlyingArrow_C" (`KismetMathLibrary.MakeTransform` (`self.K2_GetActorLocation`) (`self.K2_GetActorRotation`)) "Undefined" "MultiplyWithRoot" null (`self.ArrowSpeed`) null))
    (`KismetSystemLibrary.Delay` 0.1)
    (`/Game/Programacion/GravStuff/Blueprints/BP_FlyingArrow.OnSpawn` _returnvalue)
    (set `self.ShootingArrows` false)))

(fn `UserConstructionScript`)