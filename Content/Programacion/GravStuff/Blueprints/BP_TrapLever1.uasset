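; Trap lever actor that toggles the display of trap 1 on the level's grid.
; A sphere overlap shows a widget, while ShowTrap1 flips IsPressed and passes it as 1 or 0 to ShowingTrap1 on the first grid actor found.
; End overlap reuses the BeginPlay chain, so leaving the sphere hides the widget, resets the lever and switches the trap display off.
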(event `self.Sphere.OnComponentBeginOverlap`
  (params (OverlappedComponent :type "PrimitiveComponent Object Reference") (OtherActor :type "Actor Object Reference") (OtherComp :type "PrimitiveComponent Object Reference") (OtherBodyIndex :type Integer) (bFromSweep :type Boolean) (SweepResult :type "HitResult Structure (by ref)"))
  (`SceneComponent.SetVisibility` (`self.Widget`) true false))

(event `self.ReceiveBeginPlay`
  (`SceneComponent.SetVisibility` (`self.Widget`) false false :!label _label)
  (set `self.IsPressed` false)
  (bind _outactors (`GameplayStatics.GetAllActorsOfClass` "/Game/Programacion/Blueprints/BP_Grid_NO_MODIFICAR_SOLO_COPIAR.BP_Grid_NO_MODIFICAR_SOLO_COPIAR_C" :!label _label_2))
  (if (`self.IsPressed`)
    (bind _output (`|GetArrayItem` _outactors))
    (`/Game/Programacion/Blueprints/BP_Grid_NO_MODIFICAR_SOLO_COPIAR.ShowingTrap1` _output 1.0)
    (else
      (`/Game/Programacion/Blueprints/BP_Grid_NO_MODIFICAR_SOLO_COPIAR.ShowingTrap1` _output 0.0))))

(event `self.Sphere.OnComponentEndOverlap`
  (params (OverlappedComponent :type "PrimitiveComponent Object Reference") (OtherActor :type "Actor Object Reference") (OtherComp :type "PrimitiveComponent Object Reference") (OtherBodyIndex :type Integer))
  (goto _label))

(event `/Game/Programacion/GravStuff/BPI_Interact.ShowTrap1`
  (if (`self.IsPressed`)
    (set `self.IsPressed` false)
    (goto _label_2)
    (else
      (set `self.IsPressed` true)
      (goto _label_2))))

(fn `UserConstructionScript`)