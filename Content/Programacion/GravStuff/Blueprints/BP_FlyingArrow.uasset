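; BP_FlyingArrow is a timed-life projectile that kills the BP_ThirdPersonCharacter it overlaps.
; BeginPlay copies its speed variables into ProjectileMovement and sets its lifespan.
; Tick runs a debug-drawn Visibility line trace from the actor to its End component, but nothing acts on the result.
; Impact effect, shade spawning and destroy-on-hit logic are disconnected, and the Shade function is empty.
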(event `self.ReceiveBeginPlay`
  (bind _projectilemovement (`self.ProjectileMovement`))
  (set `ProjectileMovementComponent.InitialSpeed` (`self.ArrowSpeed`) _projectilemovement)
  (set `ProjectileMovementComponent.MaxSpeed` (`self.Max Speed`) _projectilemovement)
  (`self.SetLifeSpan` (`self.arrowLifeSpan`)))

(event `self.ReceiveActorBeginOverlap`
  (params (OtherActor :type "Actor Object Reference"))
  (bind _asbp_third_person_character (cast `/Game/ThirdPerson/Blueprints/BP_ThirdPersonCharacter` OtherActor))
  (`/Game/ThirdPerson/Blueprints/BP_ThirdPersonCharacter.Die` _asbp_third_person_character))

(event `OnSpawn`)

(event `self.ReceiveTick`
  (params (DeltaSeconds :type "Float (single-precision)"))
  (bind _outhit (`KismetSystemLibrary.LineTraceSingle` :`Start` (`self.K2_GetActorLocation` (`ActorComponent.GetOwner` (`self.DefaultSceneRoot`))) :`End` (`SceneComponent.K2_GetComponentLocation` (`self.End`)) :`TraceChannel` "TraceTypeQuery1" :`DrawDebugType` "ForOneFrame" :`DrawTime` 1.0))
  (if (<= (`.Distance` (`GameplayStatics.BreakHitResult` _outhit)) 0.0)
    _))

(fn `Shade`)

(fn `UserConstructionScript`)