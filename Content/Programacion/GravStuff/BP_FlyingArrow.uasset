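; BP_FlyingArrow is a simple projectile actor that flies until it overlaps another actor or its lifespan runs out.
; BeginPlay sets the lifespan from ArrowLifeSpan, and any actor overlap destroys it.
; Each Tick offsets the root by the Arrow component's normalized forward vector times ArrowSpeed, without sweep or delta-time scaling, so speed depends on frame rate.
; The world-space forward vector is applied as a local offset.
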(event `self.ReceiveBeginPlay`
  (`self.SetLifeSpan` (`self.arrowLifeSpan`)))

(event `self.ReceiveActorBeginOverlap`
  (params (OtherActor :type "Actor Object Reference"))
  (`self.K2_DestroyActor`))

(event `self.ReceiveTick`
  (params (DeltaSeconds :type "Float (single-precision)"))
  (`SceneComponent.K2_AddLocalOffset` (`self.DefaultSceneRoot`) (* (`KismetMathLibrary.Normal` (`SceneComponent.GetForwardVector` (`self.Arrow`))) (`self.ArrowSpeed`)) false false))

(fn `UserConstructionScript`)