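; BP_ArrowSpawner is an actor that repeatedly fires BP_FlyingArrow projectiles at randomized intervals.
; Tick uses the ShootingArrows flag as a gate, so only one delayed shot is pending at a time.
; After a random delay between MinTimeInterval and MaxTimeInterval, it spawns an arrow at its own transform, passes in ArrowSpeed and reopens the gate.
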(event `self.ReceiveBeginPlay`)

(event `self.ReceiveTick`
  (params (DeltaSeconds :type "Float (single-precision)"))
  (if (not (`self.ShootingArrows`))
    (set `self.ShootingArrows` true)
    (`KismetSystemLibrary.Delay` (`KismetMathLibrary.RandomFloatInRange` (`self.minTimeInterval`) (`self.maxTimeInterval`)))
    (`|SpawnActorFromClass` "/Game/Programacion/GravStuff/BP_FlyingArrow.BP_FlyingArrow_C" (`self.GetTransform`) "Undefined" "MultiplyWithRoot" null (`self.ArrowSpeed`) null)
    (set `self.ShootingArrows` false)))

(fn `UserConstructionScript`)