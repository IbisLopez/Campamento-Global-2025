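; BP_TRapLvl3 is a level 3 flood trap whose rising water mesh threatens the player.
; Overlapping the CallingUp trigger with BP_ThirdPersonCharacter waits a configurable delay, then plays the Flood timeline at an adjustable rate.
; The timeline drives the mesh's relative Z, scaled by a configurable height.
; A separate DeathZone overlap calls Dead on BP_ThirdPersonCharacterLuis, a different character class from the trigger's cast.
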(event `self.ReceiveBeginPlay`)

(event `self.CallingUp.OnComponentBeginOverlap`
  (params (OverlappedComponent :type "PrimitiveComponent Object Reference") (OtherActor :type "Actor Object Reference") (OtherComp :type "PrimitiveComponent Object Reference") (OtherBodyIndex :type Integer) (bFromSweep :type Boolean) (SweepResult :type "HitResult Structure (by ref)"))
  ; trap  to go up
  (cast `/Game/ThirdPerson/Blueprints/BP_ThirdPersonCharacter` OtherActor)
  (`KismetSystemLibrary.Delay` (`self.Duration to water start go up`))
  (`TimelineComponent.SetPlayRate` (`self.Flood`) (`self.how fast?`))
  ;; time to go up
  (bind (_direction _filledup) (`Timeline|Flood`)
    (:`Update`
      (`SceneComponent.K2_SetRelativeLocation` (`self.StaticMesh`) (`KismetMathLibrary.MakeVector` 0.0 0.0 (* _filledup (`self.How Up?`))) false false))))

(event `self.deathZone.OnComponentBeginOverlap`
  (params (OverlappedComponent :type "PrimitiveComponent Object Reference") (OtherActor :type "Actor Object Reference") (OtherComp :type "PrimitiveComponent Object Reference") (OtherBodyIndex :type Integer) (bFromSweep :type Boolean) (SweepResult :type "HitResult Structure (by ref)"))
  (bind _asbp_third_person_character_luis (cast `/Game/ThirdPerson/Blueprints/BP_ThirdPersonCharacterLuis` OtherActor))
  (`/Game/ThirdPerson/Blueprints/BP_ThirdPersonCharacterLuis.Dead` _asbp_third_person_character_luis))

(fn `UserConstructionScript`)