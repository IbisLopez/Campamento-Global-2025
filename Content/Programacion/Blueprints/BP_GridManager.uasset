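; Grid manager that randomly picks one of five grid copy variants when play begins.
; BeginPlay rolls a random integer and calls the matching Aberracion function, storing the returned actor in that variant's GridC variable.
; Each function finds the BP_Grid_Copia actors through nested GetAllActorsOfClass loops, flags all but the chosen one as WillBeDestroyed, and records the chosen class in CopiaDelGrid.
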(event `self.ReceiveBeginPlay`
  (bind _output_get (set `self.Random` (`KismetMathLibrary.RandomInteger` 5)))
  (switch `int` _output_get
    (:`Default`
      (`KismetSystemLibrary.PrintString` "No Hay Grids"))
    (:`0`
      (bind _outactors (`GameplayStatics.GetAllActorsOfClass` "/Game/Programacion/Blueprints/Instances/BP_Grid_Copia1.BP_Grid_Copia1_C"))
      (for _array_element _outactors
        (bind _asbp_grid_copia_1 (cast `/Game/Programacion/Blueprints/Instances/BP_Grid_Copia1` _array_element))
        (set `/Game/Programacion/Blueprints/BP_Grid_NO_MODIFICAR_SOLO_COPIAR.WillBeDestroyed` false _asbp_grid_copia_1)
        (bind _outactors_2 (`GameplayStatics.GetAllActorsOfClass` "/Game/Programacion/Blueprints/Instances/BP_Grid_Copia2.BP_Grid_Copia2_C"))
        (for _array_element_2 _outactors_2
          (bind _asbp_grid_copia_2 (cast `/Game/Programacion/Blueprints/Instances/BP_Grid_Copia2` _array_element_2))
          (set `/Game/Programacion/Blueprints/BP_Grid_NO_MODIFICAR_SOLO_COPIAR.WillBeDestroyed` true _asbp_grid_copia_2)
          (bind _outactors_3 (`GameplayStatics.GetAllActorsOfClass` "/Game/Programacion/Blueprints/Instances/BP_Grid_Copia3.BP_Grid_Copia3_C"))
          (for _array_element_3 _outactors_3
            (bind _asbp_grid_copia_3 (cast `/Game/Programacion/Blueprints/Instances/BP_Grid_Copia3` _array_element_3))
            (set `/Game/Programacion/Blueprints/BP_Grid_NO_MODIFICAR_SOLO_COPIAR.WillBeDestroyed` true _asbp_grid_copia_3)
            (bind _outactors_4 (`GameplayStatics.GetAllActorsOfClass` "/Game/Programacion/Blueprints/Instances/BP_Grid_Copia4.BP_Grid_Copia4_C"))
            (for _array_element_4 _outactors_4
              (bind _asbp_grid_copia_4 (cast `/Game/Programacion/Blueprints/Instances/BP_Grid_Copia4` _array_element_4))
              (set `/Game/Programacion/Blueprints/BP_Grid_NO_MODIFICAR_SOLO_COPIAR.WillBeDestroyed` true _asbp_grid_copia_4)
              (bind _outactors_5 (`GameplayStatics.GetAllActorsOfClass` "/Game/Programacion/Blueprints/Instances/BP_Grid_Copia5.BP_Grid_Copia5_C"))
              (for _array_element_5 _outactors_5
                (bind _asbp_grid_copia_5 (cast `/Game/Programacion/Blueprints/Instances/BP_Grid_Copia5` _array_element_5))
                (set `/Game/Programacion/Blueprints/BP_Grid_NO_MODIFICAR_SOLO_COPIAR.WillBeDestroyed` true _asbp_grid_copia_5)
                (set `self.CopiaDelGrid` (`GameplayStatics.GetObjectClass` _asbp_grid_copia_1))
                (set `self.Grid C1` _asbp_grid_copia_1)))))))
    (:`1`
      (bind _outactors_6 (`GameplayStatics.GetAllActorsOfClass` "/Game/Programacion/Blueprints/Instances/BP_Grid_Copia1.BP_Grid_Copia1_C"))
      (for _array_element_6 _outactors_6
        (bind _asbp_grid_copia_1_2 (cast `/Game/Programacion/Blueprints/Instances/BP_Grid_Copia1` _array_element_6))
        (set `/Game/Programacion/Blueprints/BP_Grid_NO_MODIFICAR_SOLO_COPIAR.WillBeDestroyed` true _asbp_grid_copia_1_2)
        (bind _outactors_7 (`GameplayStatics.GetAllActorsOfClass` "/Game/Programacion/Blueprints/Instances/BP_Grid_Copia2.BP_Grid_Copia2_C"))
        (for _array_element_7 _outactors_7
          (bind _asbp_grid_copia_2_2 (cast `/Game/Programacion/Blueprints/Instances/BP_Grid_Copia2` _array_element_7))
          (set `/Game/Programacion/Blueprints/BP_Grid_NO_MODIFICAR_SOLO_COPIAR.WillBeDestroyed` false _asbp_grid_copia_2_2)
          (bind _outactors_8 (`GameplayStatics.GetAllActorsOfClass` "/Game/Programacion/Blueprints/Instances/BP_Grid_Copia3.BP_Grid_Copia3_C"))
          (for _array_element_8 _outactors_8
            (bind _asbp_grid_copia_3_2 (cast `/Game/Programacion/Blueprints/Instances/BP_Grid_Copia3` _array_element_8))
            (set `/Game/Programacion/Blueprints/BP_Grid_NO_MODIFICAR_SOLO_COPIAR.WillBeDestroyed` true _asbp_grid_copia_3_2)
            (bind _outactors_9 (`GameplayStatics.GetAllActorsOfClass` "/Game/Programacion/Blueprints/Instances/BP_Grid_Copia4.BP_Grid_Copia4_C"))
            (for _array_element_9 _outactors_9
              (bind _asbp_grid_copia_4_2 (cast `/Game/Programacion/Blueprints/Instances/BP_Grid_Copia4` _array_element_9))
              (set `/Game/Programacion/Blueprints/BP_Grid_NO_MODIFICAR_SOLO_COPIAR.WillBeDestroyed` true _asbp_grid_copia_4_2)
              (bind _outactors_10 (`GameplayStatics.GetAllActorsOfClass` "/Game/Programacion/Blueprints/Instances/BP_Grid_Copia5.BP_Grid_Copia5_C"))
              (for _array_element_10 _outactors_10
                (bind _asbp_grid_copia_5_2 (cast `/Game/Programacion/Blueprints/Instances/BP_Grid_Copia5` _array_element_10))
                (set `/Game/Programacion/Blueprints/BP_Grid_NO_MODIFICAR_SOLO_COPIAR.WillBeDestroyed` true _asbp_grid_copia_5_2)
                (set `self.CopiaDelGrid` (`GameplayStatics.GetObjectClass` _asbp_grid_copia_2_2))
                (set `self.Grid C2` _asbp_grid_copia_2_2)))))))
    (:`2`
      (bind _outactors_11 (`GameplayStatics.GetAllActorsOfClass` "/Game/Programacion/Blueprints/Instances/BP_Grid_Copia1.BP_Grid_Copia1_C"))
      (for _array_element_11 _outactors_11
        (bind _asbp_grid_copia_1_3 (cast `/Game/Programacion/Blueprints/Instances/BP_Grid_Copia1` _array_element_11))
        (set `/Game/Programacion/Blueprints/BP_Grid_NO_MODIFICAR_SOLO_COPIAR.WillBeDestroyed` true _asbp_grid_copia_1_3)
        (bind _outactors_12 (`GameplayStatics.GetAllActorsOfClass` "/Game/Programacion/Blueprints/Instances/BP_Grid_Copia2.BP_Grid_Copia2_C"))
        (for _array_element_12 _outactors_12
          (bind _asbp_grid_copia_2_3 (cast `/Game/Programacion/Blueprints/Instances/BP_Grid_Copia2` _array_element_12))
          (set `/Game/Programacion/Blueprints/BP_Grid_NO_MODIFICAR_SOLO_COPIAR.WillBeDestroyed` true _asbp_grid_copia_2_3)
          (bind _outactors_13 (`GameplayStatics.GetAllActorsOfClass` "/Game/Programacion/Blueprints/Instances/BP_Grid_Copia3.BP_Grid_Copia3_C"))
          (for _array_element_13 _outactors_13
            (bind _asbp_grid_copia_3_3 (cast `/Game/Programacion/Blueprints/Instances/BP_Grid_Copia3` _array_element_13))
            (set `/Game/Programacion/Blueprints/BP_Grid_NO_MODIFICAR_SOLO_COPIAR.WillBeDestroyed` false _asbp_grid_copia_3_3)
            (bind _outactors_14 (`GameplayStatics.GetAllActorsOfClass` "/Game/Programacion/Blueprints/Instances/BP_Grid_Copia4.BP_Grid_Copia4_C"))
            (for _array_element_14 _outactors_14
              (bind _asbp_grid_copia_4_3 (cast `/Game/Programacion/Blueprints/Instances/BP_Grid_Copia4` _array_element_14))
              (set `/Game/Programacion/Blueprints/BP_Grid_NO_MODIFICAR_SOLO_COPIAR.WillBeDestroyed` true _asbp_grid_copia_4_3)
              (bind _outactors_15 (`GameplayStatics.GetAllActorsOfClass` "/Game/Programacion/Blueprints/Instances/BP_Grid_Copia5.BP_Grid_Copia5_C"))
              (for _array_element_15 _outactors_15
                (bind _asbp_grid_copia_5_3 (cast `/Game/Programacion/Blueprints/Instances/BP_Grid_Copia5` _array_element_15))
                (set `/Game/Programacion/Blueprints/BP_Grid_NO_MODIFICAR_SOLO_COPIAR.WillBeDestroyed` true _asbp_grid_copia_5_3)
                (set `self.CopiaDelGrid` (`GameplayStatics.GetObjectClass` _asbp_grid_copia_3_3))
                (set `self.Grid C3` _asbp_grid_copia_3_3)))))))
    (:`3`
      (bind _outactors_16 (`GameplayStatics.GetAllActorsOfClass` "/Game/Programacion/Blueprints/Instances/BP_Grid_Copia1.BP_Grid_Copia1_C"))
      (for _array_element_16 _outactors_16
        (bind _asbp_grid_copia_1_4 (cast `/Game/Programacion/Blueprints/Instances/BP_Grid_Copia1` _array_element_16))
        (set `/Game/Programacion/Blueprints/BP_Grid_NO_MODIFICAR_SOLO_COPIAR.WillBeDestroyed` true _asbp_grid_copia_1_4)
        (bind _outactors_17 (`GameplayStatics.GetAllActorsOfClass` "/Game/Programacion/Blueprints/Instances/BP_Grid_Copia2.BP_Grid_Copia2_C"))
        (for _array_element_17 _outactors_17
          (bind _asbp_grid_copia_2_4 (cast `/Game/Programacion/Blueprints/Instances/BP_Grid_Copia2` _array_element_17))
          (set `/Game/Programacion/Blueprints/BP_Grid_NO_MODIFICAR_SOLO_COPIAR.WillBeDestroyed` true _asbp_grid_copia_2_4)
          (bind _outactors_18 (`GameplayStatics.GetAllActorsOfClass` "/Game/Programacion/Blueprints/Instances/BP_Grid_Copia3.BP_Grid_Copia3_C"))
          (for _array_element_18 _outactors_18
            (bind _asbp_grid_copia_3_4 (cast `/Game/Programacion/Blueprints/Instances/BP_Grid_Copia3` _array_element_18))
            (set `/Game/Programacion/Blueprints/BP_Grid_NO_MODIFICAR_SOLO_COPIAR.WillBeDestroyed` true _asbp_grid_copia_3_4)
            (bind _outactors_19 (`GameplayStatics.GetAllActorsOfClass` "/Game/Programacion/Blueprints/Instances/BP_Grid_Copia4.BP_Grid_Copia4_C"))
            (for _array_element_19 _outactors_19
              (bind _asbp_grid_copia_4_4 (cast `/Game/Programacion/Blueprints/Instances/BP_Grid_Copia4` _array_element_19))
              (set `/Game/Programacion/Blueprints/BP_Grid_NO_MODIFICAR_SOLO_COPIAR.WillBeDestroyed` false _asbp_grid_copia_4_4)
              (bind _outactors_20 (`GameplayStatics.GetAllActorsOfClass` "/Game/Programacion/Blueprints/Instances/BP_Grid_Copia5.BP_Grid_Copia5_C"))
              (for _array_element_20 _outactors_20
                (bind _asbp_grid_copia_5_4 (cast `/Game/Programacion/Blueprints/Instances/BP_Grid_Copia5` _array_element_20))
                (set `/Game/Programacion/Blueprints/BP_Grid_NO_MODIFICAR_SOLO_COPIAR.WillBeDestroyed` true _asbp_grid_copia_5_4)
                (set `self.CopiaDelGrid` (`GameplayStatics.GetObjectClass` _asbp_grid_copia_4_4))
                (set `self.Grid C4` _asbp_grid_copia_4_4)))))))
    (:`4`
      (bind _outactors_21 (`GameplayStatics.GetAllActorsOfClass` "/Game/Programacion/Blueprints/Instances/BP_Grid_Copia1.BP_Grid_Copia1_C"))
      (for _array_element_21 _outactors_21
        (bind _asbp_grid_copia_1_5 (cast `/Game/Programacion/Blueprints/Instances/BP_Grid_Copia1` _array_element_21))
        (set `/Game/Programacion/Blueprints/BP_Grid_NO_MODIFICAR_SOLO_COPIAR.WillBeDestroyed` true _asbp_grid_copia_1_5)
        (bind _outactors_22 (`GameplayStatics.GetAllActorsOfClass` "/Game/Programacion/Blueprints/Instances/BP_Grid_Copia2.BP_Grid_Copia2_C"))
        (for _array_element_22 _outactors_22
          (bind _asbp_grid_copia_2_5 (cast `/Game/Programacion/Blueprints/Instances/BP_Grid_Copia2` _array_element_22))
          (set `/Game/Programacion/Blueprints/BP_Grid_NO_MODIFICAR_SOLO_COPIAR.WillBeDestroyed` true _asbp_grid_copia_2_5)
          (bind _outactors_23 (`GameplayStatics.GetAllActorsOfClass` "/Game/Programacion/Blueprints/Instances/BP_Grid_Copia3.BP_Grid_Copia3_C"))
          (for _array_element_23 _outactors_23
            (bind _asbp_grid_copia_3_5 (cast `/Game/Programacion/Blueprints/Instances/BP_Grid_Copia3` _array_element_23))
            (set `/Game/Programacion/Blueprints/BP_Grid_NO_MODIFICAR_SOLO_COPIAR.WillBeDestroyed` true _asbp_grid_copia_3_5)
            (bind _outactors_24 (`GameplayStatics.GetAllActorsOfClass` "/Game/Programacion/Blueprints/Instances/BP_Grid_Copia4.BP_Grid_Copia4_C"))
            (for _array_element_24 _outactors_24
              (bind _asbp_grid_copia_4_5 (cast `/Game/Programacion/Blueprints/Instances/BP_Grid_Copia4` _array_element_24))
              (set `/Game/Programacion/Blueprints/BP_Grid_NO_MODIFICAR_SOLO_COPIAR.WillBeDestroyed` true _asbp_grid_copia_4_5)
              (bind _outactors_25 (`GameplayStatics.GetAllActorsOfClass` "/Game/Programacion/Blueprints/Instances/BP_Grid_Copia5.BP_Grid_Copia5_C"))
              (for _array_element_25 _outactors_25
                (bind _asbp_grid_copia_5_5 (cast `/Game/Programacion/Blueprints/Instances/BP_Grid_Copia5` _array_element_25))
                (set `/Game/Programacion/Blueprints/BP_Grid_NO_MODIFICAR_SOLO_COPIAR.WillBeDestroyed` false _asbp_grid_copia_5_5)
                (set `self.CopiaDelGrid` (`GameplayStatics.GetObjectClass` _asbp_grid_copia_5_5))
                (set `self.Grid C5` _asbp_grid_copia_5_5)))))))))

(fn `UserConstructionScript`)